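; Rathalos monster Blueprint that tracks health, a current state and a breakable tail.
; On BeginPlay it fills HP to max and sets an initial enum state.
; RecieveHit applies damage to HP and routes hits on tail bones 02 to 05 into a separate durability pool at a tenfold multiplier.
; Death and tail severing only set one-time flags and print debug messages.
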(event Custom|RecieveHit
  (params (Damage :type Float%20%28double-precision%29) (Bone :type Name))
  (CallFunction|ApplyMonsterHP Damage)
  (switch name Bone
    (:Tail_02
      _)
    (:Tail_03
      _)
    (:Tail_04
      _)
    (:Tail_05
      _))
  (CallFunction|ApplyTailDurability Damage))

(event EventBeginPlay
  (Variables|Default|SetCurHp (Variables|Default|GetMaxHP))
  (CallFunction|SetMonsetState "NewEnumerator2"))

(event Collision|EventActorBeginOverlap
  (params (OtherActor :type Actor%20Object%20Reference)))

(event EventTick
  (params (DeltaSeconds :type Float%20%28single-precision%29)))

(fn ConstructionScript)

(fn SetMonsetState
  (params (NewParam :type E_MonsterState%20Enum :default "NewEnumerator0"))
  (Variables|Default|SetCurrentState NewParam))

(fn ApplyMonsterHP
  (params (Damage :type Float%20%28double-precision%29))
  (if (Variables|Default|GetIsAlive)
    (Variables|Default|SetCurHp (- (Variables|Default|GetCurHp) Damage))
    (if (<= (Variables|Default|GetCurHp) 0.0)
      (Variables|Default|SetCurHp 0.0)
      (Variables|Default|SetIsAlive false)
      (Development|PrintString "사망"))))

(fn ApplyTailDurability
  (params (Damage :type Float%20%28double-precision%29))
  (if (not (Variables|Default|GetIsTailDestroyed))
    (Variables|Default|SetTailDurability (- (Variables|Default|GetTailDurability) (* Damage 1e+01)))
    (if (<= (Variables|Default|GetTailDurability) 0.0)
      (Variables|Default|SetIsTailDestroyed true)
      (Development|PrintString "꼬짤"))))